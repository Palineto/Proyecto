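; Saloon door Blueprint that the player swings open and closed with the E key.
; Overlap begin and end enable and disable input for player controller 0, with no check on which actor overlaps.
; Each press flips the DoorStatus boolean and plays or reverses a timeline, whose track sets the relative yaw of the Cube component.
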(event `Key|E`
  (params (Key :type "Key Structure" :default "AnyKey"))
  (:`Pressed`
    (if (`self.Door Status`)
      (set `self.Door Status` false)
      (bind (_direction _newtrack_0) (`Timeline|Timeline_0` :!via `Reverse` :!label _label)
        (:`Update`
          (`SceneComponent.K2_SetRelativeRotation` (`self.Cube`) (`KismetMathLibrary.MakeRotator` 0.0 0.0 _newtrack_0) false false)))
      (else
        (set `self.Door Status` true)
        (goto _label)))))

(event `self.ReceiveActorBeginOverlap`
  (params (OtherActor :type "Actor Object Reference"))
  (`self.EnableInput` (`GameplayStatics.GetPlayerController` 0)))

(event `self.ReceiveActorEndOverlap`
  (params (OtherActor :type "Actor Object Reference"))
  (`self.DisableInput` (`GameplayStatics.GetPlayerController` 0)))

(fn `UserConstructionScript`)